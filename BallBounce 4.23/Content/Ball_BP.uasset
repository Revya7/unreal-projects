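; Ball Blueprint for a physics-driven ball that keeps moving at a set speed as it bounces.
; LaunchBall sets a diagonal starting velocity from BallSpeed.
; On each hit, it clamps the linear velocity's magnitude to BallSpeed, passes it through CalculateRotator, and applies the rotated result, correcting speed and angle without using Tick.
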(event `self.ReceiveBeginPlay`)

(event `LaunchBall`
  (bind _ballspeed (`self.ballSpeed`))
  ;[1 1 1] LaunchBall
  (`PrimitiveComponent.SetPhysicsLinearVelocity` (`self.Ball`) (`KismetMathLibrary.MakeVector` _ballspeed (* _ballspeed -1.0)) false "None"))

(event `self.Ball.OnComponentHit`
  (params (HitComponent :type "PrimitiveComponent Object Reference") (OtherActor :type "Actor Object Reference") (OtherComp :type "PrimitiveComponent Object Reference") (NormalImpulse :type "Vector Structure") (Hit :type "HitResult Structure (by ref)"))
  (bind _ballspeed (`self.ballSpeed`))
  ;[1 1 1] AdjustSpeedAndAngle
  (bind _returnvalue (`PrimitiveComponent.GetPhysicsLinearVelocity` (`self.Ball`) "None"))
  (bind (_rotateby _returnvalue_2) (`self.CalculateRotator` (`KismetMathLibrary.ClampVectorSize` _returnvalue _ballspeed _ballspeed)))
  (`PrimitiveComponent.SetPhysicsLinearVelocity` (`self.Ball`) (`KismetMathLibrary.GreaterGreater_VectorRotator` _returnvalue_2 _rotateby) false "None"))

(fn `UserConstructionScript`)