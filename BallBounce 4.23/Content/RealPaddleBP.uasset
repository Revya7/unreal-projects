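; Player paddle Blueprint that moves on input and holds and launches a ball.
; On BeginPlay it passes its BallPosition component to BallPositionArrow, then spawns a Ball_BP at that transform and stores it as MyBall.
; The Move axis feeds HandleMovement, noted as C++ movement handling.
; The LaunchBall action launches the stored ball, with IsBallLaunched blocking repeat launches.
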(event `self.ReceiveBeginPlay`
  (set `self.ballPositionArrow` (`self.BallPosition`))
  (`self.SpawnBall`))

(event `SpawnBall`
  ;[1 1 1] SpawnBall
  (bind _returnvalue (`|SpawnActorFromClass` "/Game/Ball_BP.Ball_BP_C" (`SceneComponent.K2_GetComponentToWorld` (`self.BallPosition`)) "Undefined" "OverrideRootScale" null null))
  (set `self.myBall` _returnvalue))

(event `InputAxis|Move`
  (params (AxisValue :type "Float (single-precision)"))
  ;[1 1 1] Handling Movement C++
  (`self.HandleMovement` AxisValue))

(event `InputAction|LaunchBall`
  (params (Key :type "Key Structure"))
  ;[1 1 1] LaunchBall
  (:`Pressed`
    (if (not (`self.isBallLaunched`))
      (bind _asball_bp (cast `/Game/Ball_BP` (`self.myBall`)))
      (set `self.isBallLaunched` true)
      (`/Game/Ball_BP.LaunchBall` _asball_bp))))

(fn `UserConstructionScript`)