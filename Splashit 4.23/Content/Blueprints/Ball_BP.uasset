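; Player-controlled ball that slides along the world X and Y axes, with each move consuming one from a move budget.
; BeginPlay counts the Ground_BP actors into TotalGrounds and enables input.
; A direction press, gated by CanMove, disables input, sets that direction's flag and calls DecreaseMaxMoves.
; Tick applies frame-rate-independent, unswept offsets at InitialSpeed while a flag is set; nothing in these graphs clears flags or restores movement.
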(event `self.ReceiveBeginPlay`
  (`|ExecutionSequence`
    (:`then_0`
      (bind _outactors (`GameplayStatics.GetAllActorsOfClass` "/Game/Blueprints/Ground_BP.Ground_BP_C"))
      (set `self.TotalGrounds` (`KismetArrayLibrary.Array_Length` _outactors)))
    (:`then_1`
      (`self.EnableInput` (`GameplayStatics.GetPlayerController` 0)))))

(event `InputAction|Move Right`
  (params (Key :type "Key Structure"))
  (:`Pressed`
    (if (`self.CanMove`)
      (`self.DisableInput` null)
      (set `self.CanMove` false)
      (set `self.MoveRight` true)
      (`self.DecreaseMaxMoves`))))

(event `InputAction|Move Left`
  (params (Key :type "Key Structure"))
  (:`Pressed`
    (if (`self.CanMove`)
      (`self.DisableInput` null)
      (set `self.CanMove` false)
      (set `self.MoveLeft` true)
      (`self.DecreaseMaxMoves`))))

(event `InputAction|Move Up`
  (params (Key :type "Key Structure"))
  (:`Pressed`
    (if (`self.CanMove`)
      (`self.DisableInput` null)
      (set `self.CanMove` false)
      (set `self.MoveUp` true)
      (`self.DecreaseMaxMoves`))))

(event `InputAction|Move Down`
  (params (Key :type "Key Structure"))
  (:`Pressed`
    (if (`self.CanMove`)
      (`self.DisableInput` null)
      (set `self.CanMove` false)
      (set `self.MoveDown` true)
      (`self.DecreaseMaxMoves`))))

(event `self.ReceiveTick`
  (params (DeltaSeconds :type "Float (single-precision)"))
  (bind _returnvalue (* (`GameplayStatics.GetWorldDeltaSeconds`) (`self.InitialSpeed`)))
  (bind _returnvalue_2 (* (`GameplayStatics.GetWorldDeltaSeconds`) (`self.InitialSpeed`) -1.0))
  (`|ExecutionSequence`
    (:`then_0`
      (if (`self.MoveRight`)
        (`self.K2_AddActorWorldOffset` (`KismetMathLibrary.MakeVector` _returnvalue))))
    (:`then_1`
      (if (`self.MoveDown`)
        (`self.K2_AddActorWorldOffset` (`KismetMathLibrary.MakeVector` 0.0 _returnvalue))))
    (:`then_2`
      (if (`self.MoveLeft`)
        (`self.K2_AddActorWorldOffset` (`KismetMathLibrary.MakeVector` _returnvalue_2))))
    (:`then_3`
      (if (`self.MoveUp`)
        (`self.K2_AddActorWorldOffset` (`KismetMathLibrary.MakeVector` 0.0 _returnvalue_2))))))

(fn `UserConstructionScript`)