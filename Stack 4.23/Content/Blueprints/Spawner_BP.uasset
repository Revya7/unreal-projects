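; Spawner Blueprint that creates the TileReminder piece for the offset between a current and previous tile, apparently for a tile-stacking game.
; On BeginPlay it passes its right and left arrows to SetArrowsReference.
; SpawnReminder scales the piece's X by the absolute offset and places it at the previous tile's X extent, signed by the offset, taking other axes from the current tile.
; Only movement along X is handled.
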(event `self.ReceiveBeginPlay`
  (`self.SetArrowsReference` (`self.RightArrow`) (`self.LeftArrow`)))

(event `self.SpawnReminder`
  (params (CurrentTile :type "Tile Object Reference") (PreviousTile :type "Tile Object Reference") (DifferencePosition :type "Float (single-precision)") (IsMovingX :type Boolean))
  (if IsMovingX
    (`|SpawnActorFromClass` "/Game/Blueprints/TileReminder.TileReminder_C" (`KismetMathLibrary.MakeTransform` (`KismetMathLibrary.MakeVector` (* (.x (`.BoxExtent` (`self.GetActorBounds` PreviousTile false))) (`KismetMathLibrary.SignOfFloat` DifferencePosition)) (.y (`self.K2_GetActorLocation` CurrentTile)) (.z (`self.K2_GetActorLocation` CurrentTile))) (struct) (`KismetMathLibrary.MakeVector` (`KismetMathLibrary.Abs` DifferencePosition) (.y (`self.GetActorScale3D` CurrentTile)) (.z (`self.GetActorScale3D` CurrentTile)))) "Undefined" "OverrideRootScale" null null)))

(fn `UserConstructionScript`)