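; Openable door actor that swings open and closed in response to events from its OpenDoor component.
; It stores its starting rotation on BeginPlay, then a timeline drives a yaw offset combined with that rotation each update.
; Closing plays the same timeline in reverse.
; A timeline event track times a door lock sound at the actor's location.
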(event `self.ReceiveBeginPlay`
  (set `self.Initial Rotation` (`self.K2_GetActorRotation`)))

(event `self.OpenDoor.OpenDoorEvent`
  (bind (_direction _opendoor_graph) (`Timeline|For Open Door Event` :!label _label)
    (:`Update`
      (`self.K2_SetActorRotation` (`KismetMathLibrary.ComposeRotators` (`KismetMathLibrary.MakeRotator` 0.0 0.0 _opendoor_graph) (`self.Initial Rotation`))))
    (:`Sound Timing Event`
      (`GameplayStatics.PlaySoundAtLocation` "/Game/Audiozz/door-lock.door-lock" (`self.K2_GetActorLocation`) (struct) 1.0 1.0 0.0 null null null))))

(event `self.OpenDoor.CloseDoorEvent`
  (goto _label :!via `Reverse`))

(fn `UserConstructionScript`)